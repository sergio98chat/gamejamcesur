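; BP_Generator spawns clothing Blueprints at the level's item spawn points when play begins.
; It queries the Asset Registry for assets in the Clothes folder, non-recursively, and stores them in ClothesArray.
; Each BP_ItemSpawnPoints actor takes the asset at its own index, with no shuffling or bounds check.
; The generated class is blocking-loaded by appending "_C" to the asset path, then spawned at that point's transform.
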(event `self.ReceiveBeginPlay`
  (bind (_outassetdata _returnvalue) (`AssetRegistry.GetAssetsByPath` (`AssetRegistryHelpers.GetAssetRegistry`) "/Game/Blueprints/Clothes" false false))
  (if _returnvalue
    (`KismetSystemLibrary.PrintString` (`KismetStringLibrary.Conv_IntToString` (`KismetArrayLibrary.Array_LastIndex` _outassetdata)))
    (bind _output_get (set `self.ClothesArray` _outassetdata))
    (bind _outactors (`GameplayStatics.GetAllActorsOfClass` "/Game/Blueprints/Generator/BP_ItemSpawnPoints.BP_ItemSpawnPoints_C"))
    (if (`KismetArrayLibrary.Array_IsNotEmpty` _outactors)
      (for (_array_element _array_index) _outactors
        (bind _returnvalue_2 (`KismetSystemLibrary.LoadClassAsset_Blocking` (`KismetSystemLibrary.Conv_SoftClassPathToSoftClassRef` (`KismetSystemLibrary.MakeSoftClassPath` (`KismetStringLibrary.Concat_StrStr` (`KismetSystemLibrary.GetPathName` (`AssetRegistryHelpers.GetAsset` (`|GetArrayItem` _output_get _array_index))) "_C")))))
        (bind _asactor (castclass `Actor` _returnvalue_2))
        (`|SpawnActorFromClass` _asactor (`self.GetTransform` _array_element) "AdjustIfPossibleButAlwaysSpawn" "MultiplyWithRoot" null null)))))

(fn `UserConstructionScript`)