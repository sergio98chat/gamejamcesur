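; BP_BlusaMuher is a clothing pickup that dresses the player in the woman's blouse when they walk into its trigger box.
; On BeginPlay it caches the player's BlusaMujer piece from BP_jugador.
; On overlap by the player, it hides ChalecoPobre, shows the blouse and calls CamisetaMessage on the player's CheckBoxWidget.
; Rather than being destroyed, only the box is moved to a fixed world location below the origin.
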(event `self.ReceiveBeginPlay`
  (bind _asbp_jugador (cast `/Game/ThirdPerson/Blueprints/BP_jugador` (`GameplayStatics.GetPlayerCharacter` 0)))
  (set `self.ClothingPiece` (`/Game/ThirdPerson/Blueprints/BP_jugador.Blusa_Mujer` _asbp_jugador)))

(event `self.Box.OnComponentBeginOverlap`
  (params (OverlappedComponent :type "PrimitiveComponent Object Reference") (OtherActor :type "Actor Object Reference") (OtherComp :type "PrimitiveComponent Object Reference") (OtherBodyIndex :type Integer) (bFromSweep :type Boolean) (SweepResult :type "HitResult Structure (by ref)"))
  (if (== OtherActor (`GameplayStatics.GetPlayerCharacter` 0))
    (bind _asbp_jugador (cast `/Game/ThirdPerson/Blueprints/BP_jugador` OtherActor))
    (`/Game/ThirdPerson/Blueprints/BP_jugador.SetClothesInvisible` _asbp_jugador (`/Game/ThirdPerson/Blueprints/BP_jugador.Chaleco_Pobre` _asbp_jugador))
    (`/Game/ThirdPerson/Blueprints/BP_jugador.SetClothesVisible` _asbp_jugador (`self.ClothingPiece`))
    (`SceneComponent.K2_SetWorldLocation` (`self.Box`) (0.0 0.0 -200.0) false false)
    (message `/Game/Blueprints/CheckList/BPI_VisibleCheck.Camiseta` (`/Game/ThirdPerson/Blueprints/BP_jugador.CheckBoxWidget` _asbp_jugador))))

(fn `UserConstructionScript`
  (`parent.UserConstructionScript`))