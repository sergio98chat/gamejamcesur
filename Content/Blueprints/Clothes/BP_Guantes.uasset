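; BP_Guantes is a clothing actor for gloves that the player obtains by walking into its Box trigger.
; On BeginPlay it caches the player character's GuantesMujer piece from BP_jugador as its ClothingPiece.
; When that character overlaps the box, it passes the piece to SetClothesVisible and calls GuantesMessage on the player's CheckBoxWidget.
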(event `self.ReceiveBeginPlay`
  (bind _asbp_jugador (cast `/Game/ThirdPerson/Blueprints/BP_jugador` (`GameplayStatics.GetPlayerCharacter` 0)))
  (set `self.ClothingPiece` (`/Game/ThirdPerson/Blueprints/BP_jugador.Guantes_Mujer` _asbp_jugador)))

(event `self.Box.OnComponentBeginOverlap`
  (params (OverlappedComponent :type "PrimitiveComponent Object Reference") (OtherActor :type "Actor Object Reference") (OtherComp :type "PrimitiveComponent Object Reference") (OtherBodyIndex :type Integer) (bFromSweep :type Boolean) (SweepResult :type "HitResult Structure (by ref)"))
  (if (== OtherActor (`GameplayStatics.GetPlayerCharacter` 0))
    (bind _asbp_jugador (cast `/Game/ThirdPerson/Blueprints/BP_jugador` OtherActor))
    (`/Game/ThirdPerson/Blueprints/BP_jugador.SetClothesVisible` _asbp_jugador (`self.ClothingPiece`))
    (message `/Game/Blueprints/CheckList/BPI_VisibleCheck.Guantes` (`/Game/ThirdPerson/Blueprints/BP_jugador.CheckBoxWidget` _asbp_jugador))))

(fn `UserConstructionScript`
  (`parent.UserConstructionScript`))