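; BP_Door is a door actor that responds to an OpenDoor event based on a key count (Cuantasllavestienes) and a HasLock flag.
; With at least one key, a timeline drives the mesh's world yaw only if HasLock is set; otherwise nothing happens.
; With no key, a second timeline rotates the same mesh, regardless of HasLock.
; CloseDoor is an empty stub.
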(event `OpenDoor`
  (if (>= (`self.cuantasllavestienes?`) 1)
    (if (`self.HasLock?`)
      (bind (_direction _zrotation) (`Timeline|Timeline`)
        (:`Update`
          (`SceneComponent.K2_SetWorldRotation` (`self.StaticMesh`) (`KismetMathLibrary.MakeRotator` 0.0 0.0 _zrotation) false false))))
    (else
      (bind (_direction_2 _zrotation_2) (`Timeline|Timeline_0`)
        (:`Update`
          (`SceneComponent.K2_SetWorldRotation` (`self.StaticMesh`) (`KismetMathLibrary.MakeRotator` 0.0 0.0 _zrotation_2) false false))))))

(event `CloseDoor`)

(fn `UserConstructionScript`)